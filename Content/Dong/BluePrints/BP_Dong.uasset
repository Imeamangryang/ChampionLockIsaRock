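; BP_Dong is a character Blueprint for a TFT-style game, linking player input and movement to the TFT economy.
; On BeginPlay it caches the first TFTPlayerState and grants it starting gold, then the C key calls BuyXP on that state.
; Every Tick it searches the world for TFT_Coin actors, tripling walk speed while any exist and restoring it otherwise.
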(event `Key|C`
  (params (Key :type "Key Structure"))
  (:`Pressed`
    (`TFTPlayerState.BuyXP` (stale `self.ReceiveBeginPlay` _astftplayer_state))))

(event `self.ReceiveBeginPlay`
  (bind _astftplayer_state (cast `TFTPlayerState` (`GameplayStatics.GetPlayerState` 0)))
  (`TFTPlayerState.AddGold` _astftplayer_state 99))

(event `self.ReceiveTick`
  (params (DeltaSeconds :type "Float (single-precision)"))
  (bind _outactors (`GameplayStatics.GetAllActorsOfClass` "/Script/ChampionLockIsaRock.TFT_Coin"))
  (if (>= (`KismetArrayLibrary.Array_Length` _outactors) 1)
    (set `CharacterMovementComponent.MaxWalkSpeed` 1800.0 (`self.CharacterMovement`))
    (else
      (set `CharacterMovementComponent.MaxWalkSpeed` 600.0 (`self.CharacterMovement`)))))

(fn `UserConstructionScript`)