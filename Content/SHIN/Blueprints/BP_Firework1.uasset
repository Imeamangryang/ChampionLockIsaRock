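; BP_Firework1 is an actor that repeatedly launches a firework particle system at its own transform on a randomized timer.
; BeginPlay picks a random initial cooldown, and Tick accumulates elapsed time until it passes that cooldown.
; It then spawns the assigned SystemTemplate at the actor's location, rotation and scale, resets the timer and rolls a new random cooldown.
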(event `self.ReceiveBeginPlay`
  (set `self.Cooldown` (`KismetMathLibrary.RandomFloatInRange` 2.0 6.0)))

(event `self.ReceiveTick`
  (params (DeltaSeconds :type "Float (single-precision)"))
  (bind (_returnvalue_location _returnvalue_rotation _returnvalue_scale) (`KismetMathLibrary.BreakTransform` (`self.GetTransform`)))
  (bind _output_get (set `self.CurrentTime` (+ (`self.CurrentTime`) DeltaSeconds)))
  (if (> _output_get (`self.Cooldown`))
    (`NiagaraFunctionLibrary.SpawnSystemAtLocation` (`self.System Template`) _returnvalue_location _returnvalue_rotation _returnvalue_scale)
    (set `self.CurrentTime` 0.0)
    (set `self.Cooldown` (`KismetMathLibrary.RandomFloatInRange` 3.0 6.0))))

(fn `UserConstructionScript`)